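; BP_NPC is an NPC the player can trade with by walking into its overlap area.
; When BP_Player begins overlapping, it sets IsTrading, registers itself as the player's Trader and shows a TextRender, rotated once to face the player's camera.
; When the overlap ends, it clears both trading references and hides the text, which also starts hidden on BeginPlay.
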(event EventBeginPlay
  (|CallParentFunction)
  (Rendering|SetVisibility (Variables|Default|GetTextRender) false false))

(event Collision|EventActorBeginOverlap
  (params (OtherActor :type Actor%20Object%20Reference))
  (|CallParentFunction OtherActor)
  (Utilities|Casting|CastToBP_Player OtherActor)
  (Variables|Default|SetIsTrading true)
  (Transformation|SetWorldRotation (Variables|Default|GetTextRender) (Math|Rotator|FindLookatRotation (Transformation|GetWorldLocation (Variables|Default|GetTextRender)) (Transformation|GetWorldLocation (Components|GetChildComponent (Variables|/Game/Blueprint/BP_Player.BP_Player_C|GetCamera (CallFunction|GetPlayer)) 0))) false false)
  (Rendering|SetVisibility (Variables|Default|GetTextRender) true false)
  (Variables|/Game/Blueprint/BP_Player.BP_Player_C|SetTrader (CallFunction|GetPlayer) self))

(event EventTick
  (params (DeltaSeconds :type Float%20%28single-precision%29))
  (|CallParentFunction DeltaSeconds))

(event Collision|EventActorEndOverlap
  (params (OtherActor :type Actor%20Object%20Reference))
  (Utilities|Casting|CastToBP_Player OtherActor)
  (Variables|Default|SetIsTrading false)
  (Rendering|SetVisibility (Variables|Default|GetTextRender) false false)
  (Variables|/Game/Blueprint/BP_Player.BP_Player_C|SetTrader (CallFunction|GetPlayer) 0))

(fn ConstructionScript
  (|CallParentFunction))