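; Player Blueprint that initializes Health and Mana on BeginPlay and handles entering and leaving a trader's shop.
; Buy blends the camera to the Trader, hides its text render and replaces all widgets with a new WBP_ShopUI.
; StopBuying blends the view back to the player, restores the text, clears widgets and has BP_PlayerController set up the player UI again.
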(event EventBeginPlay
  (|CallParentFunction)
  (Variables|Default|SetMana 50)
  (Variables|Default|SetHealth 100))

(event Collision|EventActorBeginOverlap
  (params (OtherActor :type Actor%20Object%20Reference))
  (|CallParentFunction OtherActor) ; This node is disabled and will not be called.\nDrag off pins to build functionality.
)

(event EventTick
  (params (DeltaSeconds :type Float%20%28single-precision%29))
  (|CallParentFunction DeltaSeconds) ; This node is disabled and will not be called.\nDrag off pins to build functionality.
)

(fn ConstructionScript
  (|CallParentFunction))

(fn Buy
  (bind _trader (Variables|Default|GetTrader))
  (Game|Player|SetViewTargetwithBlend (Game|GetPlayerController 0) _trader 0.5 "VTBlend_Linear" 0.0 false)
  (Rendering|SetVisibility (Variables|/Game/Blueprint/BP_NPC.BP_NPC_C|GetTextRender _trader) false false)
  (Viewport|RemoveAllWidgets)
  (bind _returnvalue (UserInterface|CreateWidget "/Game/Blueprint/WBP_ShopUI.WBP_ShopUI_C" (Game|GetPlayerController 0)))
  (UserInterface|Viewport|AddtoViewport _returnvalue 0))

(fn StopBuying
  (bind _returnvalue (Game|GetPlayerController 0))
  (Game|Player|SetViewTargetwithBlend _returnvalue self 0.5 "VTBlend_Linear" 0.0 false)
  (Rendering|SetVisibility (Variables|/Game/Blueprint/BP_NPC.BP_NPC_C|GetTextRender (Variables|Default|GetTrader)) true false)
  (Viewport|RemoveAllWidgets)
  (Default|SetPlayerUI (.AsBP%20Player%20Controller (Utilities|Casting|CastToBP_PlayerController _returnvalue))))